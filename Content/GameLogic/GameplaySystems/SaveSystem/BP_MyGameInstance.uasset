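; Game instance that holds player health, dead-enemy and collected-item lists, and saves and loads game progress.
; SaveGameToDisk copies these, the player transform and key-inventory keys into a new BP_SaveData, writing one fixed slot after each of two sequence branches.
; LoadGameFromDisk checks the slot exists, then restores the variables and keys, setting the player's transform in both branches.
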(event `SaveGameToDisk`
  (bind _saveobjectref (`self.SaveObjectRef`))
  ; SaveGameFromDisk
  (bind _returnvalue (`GameplayStatics.CreateSaveGameObject` "/Game/GameLogic/GameplaySystems/SaveSystem/BP_SaveData.BP_SaveData_C"))
  (`|ExecutionSequence`
    (:`then_0`
      (bind _output_get (set `self.SaveObjectRef` _returnvalue))
      (set `/Game/GameLogic/GameplaySystems/SaveSystem/BP_SaveData.S_PlayerHealth` (`self.CurrentHealth`) _saveobjectref)
      (set `/Game/GameLogic/GameplaySystems/SaveSystem/BP_SaveData.S_DeadEnemies` (`self.DeadEnemiesList`) _saveobjectref)
      (set `/Game/GameLogic/GameplaySystems/SaveSystem/BP_SaveData.S_CollectedItems` (`self.CollectedItemsList`) _saveobjectref)
      (set `/Game/GameLogic/GameplaySystems/SaveSystem/BP_SaveData.S_PlayerTransform` (`Actor.GetTransform` (`GameplayStatics.GetPlayerCharacter` 0)) _saveobjectref))
    (:`then_1`
      (bind _asbp_third_person_character (cast `/Game/ThirdPerson/Blueprints/BP_ThirdPersonCharacter` (`GameplayStatics.GetPlayerCharacter` 0)))
      (set `/Game/GameLogic/GameplaySystems/SaveSystem/BP_SaveData.SavedKeys` (`/Game/GameLogic/GameplaySystems/UnlockDoorsSystem/BP_KeyInventoryComponent.Keys` (`Actor.GetComponentByClass` _asbp_third_person_character "/Game/GameLogic/GameplaySystems/UnlockDoorsSystem/BP_KeyInventoryComponent.BP_KeyInventoryComponent_C")) _returnvalue)))
  (`GameplayStatics.SaveGameToSlot` _output_get "Slot1"))

(event `LoadGameFromDisk`
  ; LoadGameFromDisk
  (bind _returnvalue (`GameplayStatics.DoesSaveGameExist` "Slot1"))
  (if _returnvalue
    (bind _returnvalue_2 (`GameplayStatics.LoadGameFromSlot` "Slot1"))
    (`|ExecutionSequence`
      (:`then_0`
        (bind _asbp_save_data (cast `/Game/GameLogic/GameplaySystems/SaveSystem/BP_SaveData` _returnvalue_2))
        (set `self.CurrentHealth` (`/Game/GameLogic/GameplaySystems/SaveSystem/BP_SaveData.S_PlayerHealth` _asbp_save_data))
        (set `self.CollectedItemsList` (`/Game/GameLogic/GameplaySystems/SaveSystem/BP_SaveData.S_CollectedItems` _asbp_save_data))
        (set `self.DeadEnemiesList` (`/Game/GameLogic/GameplaySystems/SaveSystem/BP_SaveData.S_DeadEnemies` _asbp_save_data)))
      (:`then_1`
        (bind _asbp_third_person_character (cast `/Game/ThirdPerson/Blueprints/BP_ThirdPersonCharacter` (`GameplayStatics.GetPlayerCharacter` 0)))
        (set `/Game/GameLogic/GameplaySystems/UnlockDoorsSystem/BP_KeyInventoryComponent.Keys` (`/Game/GameLogic/GameplaySystems/SaveSystem/BP_SaveData.SavedKeys` _asbp_save_data) (`Actor.GetComponentByClass` _asbp_third_person_character "/Game/GameLogic/GameplaySystems/UnlockDoorsSystem/BP_KeyInventoryComponent.BP_KeyInventoryComponent_C"))))
    (`Actor.K2_SetActorTransform` (`GameplayStatics.GetPlayerCharacter` 0) (`/Game/GameLogic/GameplaySystems/SaveSystem/BP_SaveData.S_PlayerTransform` _asbp_save_data) false false)))