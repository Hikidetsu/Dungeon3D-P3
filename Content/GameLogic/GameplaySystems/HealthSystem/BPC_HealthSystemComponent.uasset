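; Health component that handles death for its owning actor, treated as the player, and restarts the dungeon game.
; On BeginPlay it binds to its own damage-received dispatcher, whose handler prints MaxHealth as current health without reducing it here.
; At zero or below, it plays a 3D death sound through the owner's audio manager component, then calls RestartGame on the dungeon game mode after a short delay.
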(event `self.ReceiveBeginPlay`
  ; Damage Logic
  (add `self.OnDamageReceived` (delegate `OnDamageReceived_Event`)))

(event `OnDamageReceived_Event`
  (bind _maxhealth (`self.MaxHealth`))
  ; Damage Logic
  (`KismetSystemLibrary.PrintString` (`KismetStringLibrary.Concat_StrStr` "Vida actual: " (`KismetStringLibrary.Conv_DoubleToString` _maxhealth)))
  (if (<= _maxhealth 0.0)
    (`/Game/AudioSystem/BPC_AudioManager.PlaySound_3D` (`Actor.GetComponentByClass` (`self.GetOwner`) "/Game/AudioSystem/BPC_AudioManager.BPC_AudioManager_C") (`self.S_Death`) (`Actor.K2_GetActorLocation` (`self.GetOwner`)) 1.0)
    (bind _asbp_gm_dungeon (cast `/Game/GameLogic/Core/BP_GM_Dungeon` (`GameplayStatics.GetGameMode`)))
    (`KismetSystemLibrary.Delay` 3.0)
    (`/Game/GameLogic/Core/BP_GM_Dungeon.RestartGame` _asbp_gm_dungeon)
    (`KismetSystemLibrary.PrintString` "Jugador ha muerto." true true (struct :`R` 1.0 :`B` 0.072545 :`A` 1.0))))