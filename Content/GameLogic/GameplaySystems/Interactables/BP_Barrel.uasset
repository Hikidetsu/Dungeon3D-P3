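; BP_Barrel is a breakable barrel that shatters, plays a crash sound and then removes itself.
; Fracture spawns an FS_MasterField at the barrel's transform, presumably to break it apart, and sets the Hit flag.
; Tick polls Hit and, through a DoOnce, plays the 3D sound via the player character's BPC_AudioManager, then destroys the actor after a short delay.
; Fracture has no caller within this Blueprint.
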(event `self.ReceiveBeginPlay`)

(event `self.ReceiveTick`
  (params (DeltaSeconds :type "Float (single-precision)"))
  (if (`self.Hit`)
    (`/Engine/EditorBlueprintResources/StandardMacros.DoOnce` false
      (:`Completed`
        (`/Game/AudioSystem/BPC_AudioManager.PlaySound_3D` (`self.GetComponentByClass` (`GameplayStatics.GetPlayerCharacter` 0) "/Game/AudioSystem/BPC_AudioManager.BPC_AudioManager_C") (`self.S_Crash`) (`self.K2_GetActorLocation`) 0.5)
        (`KismetSystemLibrary.Delay` 4.0)
        (`self.K2_DestroyActor`)))))

(fn `Fracture`
  (`|SpawnActorFromClass` "/Engine/EditorResources/FieldNodes/FS_MasterField.FS_MasterField_C" (`self.GetTransform`) "Undefined" "MultiplyWithRoot" null null)
  (set `self.Hit` true))

(fn `UserConstructionScript`)