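; BP_Chest is an interactable dungeon chest that can be opened once to give the player coins.
; Interact sets Opened, plays a pickup sound, adds coins, turns the mesh material transparent and records the Room in BP_GM_Dungeon.
; CanInteract rejects opened chests.
; The GameInstance's CollectedItemsList is checked by ActorID, restoring the opened look on BeginPlay and destroying the actor after Interact if listed.
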(event `self.ReceiveBeginPlay`
  ; LoadChest from disk
  (bind _asbp_my_game_instance (cast `/Game/GameLogic/GameplaySystems/SaveSystem/BP_MyGameInstance` (`GameplayStatics.GetGameInstance`)))
  (if (`KismetArrayLibrary.Array_Contains` (`/Game/GameLogic/GameplaySystems/SaveSystem/BP_MyGameInstance.CollectedItemsList` _asbp_my_game_instance) (`self.ActorID`))
    (set `self.bOpened` true)
    (`PrimitiveComponent.SetMaterial` (`self.cc0_chest`) 0 "/Game/Assets/Shaders/M_Transparent.M_Transparent")))

(event `/Game/GameLogic/Interfaces/BPI_Interactable.Interact`
  (params (Actor :type "Actor Object Reference"))
  (bind _room (`self.Room`))
  ; Interaction Logic
  (`|ExecutionSequence`
    (:`then_0`
      (set `self.bOpened` true)
      (`/Game/AudioSystem/BPC_AudioManager.PlaySound_3D` (`self.GetComponentByClass` Actor "/Game/AudioSystem/BPC_AudioManager.BPC_AudioManager_C") (`self.S_Pickup`) (`self.K2_GetActorLocation`) 1.5)
      (bind _asbp_third_person_character (cast `/Game/ThirdPerson/Blueprints/BP_ThirdPersonCharacter` Actor))
      (`/Game/ThirdPerson/Blueprints/BP_ThirdPersonCharacter.AddCoins` _asbp_third_person_character (`self.CoinsToGive`))
      (`PrimitiveComponent.SetMaterial` (`self.cc0_chest`) 0 "/Game/Assets/Shaders/M_Transparent.M_Transparent")
      (bind _asbp_gm_dungeon (cast `/Game/GameLogic/Core/BP_GM_Dungeon` (`GameplayStatics.GetGameMode`)))
      (`BlueprintMapLibrary.Map_Add` (`/Game/GameLogic/Core/BP_GM_Dungeon.OpenedChest` _asbp_gm_dungeon) _room true)
      (`KismetSystemLibrary.PrintString` _room))
    (:`then_1`
      (bind _asbp_my_game_instance (cast `/Game/GameLogic/GameplaySystems/SaveSystem/BP_MyGameInstance` (`GameplayStatics.GetGameInstance`)))
      (if (`KismetArrayLibrary.Array_Contains` (`/Game/GameLogic/GameplaySystems/SaveSystem/BP_MyGameInstance.CollectedItemsList` _asbp_my_game_instance) (`self.ActorID`))
        (`self.K2_DestroyActor`)))))

(fn `CanInteract`
  (params (Actor :type "Actor Object Reference"))
  (returns (CanInteract :type Boolean))
  ; Cant Interact function
  (if (`self.bOpened`)
    (return false)
    (else
      (return true))))

(fn `UserConstructionScript`)