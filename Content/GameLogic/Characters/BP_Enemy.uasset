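; Melee enemy character that spots pawns, punches the player and ragdolls on death.
; PawnSensing writes any seen pawn to the AI controller's TargetPlayer blackboard key.
; Damage plays a hit montage while Health exceeds one; a later hit triggers ragdoll and delayed destruction, with sounds routed through the player's BPC_AudioManager.
; TryPunch sphere-traces at PunchPosition to damage the player, latching PunchFlag until ResetPunchFlag allows another hit.
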(event `self.PawnSensing.OnSeePawn`
  (params (Pawn :type "Pawn Object Reference"))
  (bind _asai_controller (cast `/Game/GameLogic/IA/AI_Controller` (`self.GetController`)))
  (bind _returnvalue (`AIBlueprintHelperLibrary.GetBlackboard` _asai_controller))
  (`/Engine/EditorBlueprintResources/StandardMacros.IsValid` _returnvalue
    (:`Is Valid`
      (`BlackboardComponent.SetValueAsObject` _returnvalue "TargetPlayer" Pawn))))

(event `self.ReceiveAnyDamage`
  (params (Damage :type "Float (single-precision)") (DamageType :type "DamageType Object Reference") (InstigatedBy :type "Controller Object Reference") (DamageCauser :type "Actor Object Reference"))
  (bind _health (`self.Health`))
  (if (> _health 1.0)
    (set `self.Health` (- _health Damage))
    (`/Game/AudioSystem/BPC_AudioManager.PlaySound_3D` (`self.GetComponentByClass` (`GameplayStatics.GetPlayerCharacter` 0) "/Game/AudioSystem/BPC_AudioManager.BPC_AudioManager_C") (`self.S_hurt`) (`self.K2_GetActorLocation`) 1.0)
    (bind _returnvalue (`self.PlayAnimMontage` "/Game/Assets/Animation/Attacks/AN_Hit_Montague.AN_Hit_Montague"))
    (`KismetSystemLibrary.Delay` _returnvalue)
    (else
      (`/Game/AudioSystem/BPC_AudioManager.PlaySound_3D` (`self.GetComponentByClass` (`GameplayStatics.GetPlayerCharacter` 0) "/Game/AudioSystem/BPC_AudioManager.BPC_AudioManager_C") (`self.S_Death`) (`self.K2_GetActorLocation`) 1.0)
      (`PrimitiveComponent.SetSimulatePhysics` (`self.Mesh`) true)
      (`PrimitiveComponent.SetCollisionEnabled` (`self.CapsuleComponent`) "NoCollision")
      (`KismetSystemLibrary.Delay` 5.0)
      (`self.K2_DestroyActor`))))

(fn `GetTargetLocation`
  (returns (Location :type "Vector Structure"))
  (return (0.0 0.0 0.0)))

(fn `ResetPunchFlag`
  (set `self.punchFlag` false))

(fn `TryPunch`
  (bind _returnvalue (`self.K2_GetActorLocation`))
  (bind _returnvalue_2 (`SceneComponent.K2_GetComponentLocation` (`self.PunchPosition`)))
  (if (not (`self.punchFlag`))
    (bind _outhit (`KismetSystemLibrary.SphereTraceSingleForObjects` _returnvalue_2 _returnvalue_2 50.0 (`|MakeArray` "ObjectTypeQuery3" :!type "EObjectTypeQuery Enum")))
    (bind _asbp_third_person_character (cast `/Game/ThirdPerson/Blueprints/BP_ThirdPersonCharacter` (`.HitActor` (`GameplayStatics.BreakHitResult` _outhit))))
    (`/Game/ThirdPerson/Blueprints/BP_ThirdPersonCharacter.ApplyDamage` _asbp_third_person_character (`self.Damage to give`) _returnvalue)
    (`/Game/AudioSystem/BPC_AudioManager.PlaySound_3D` (`self.GetComponentByClass` _asbp_third_person_character "/Game/AudioSystem/BPC_AudioManager.BPC_AudioManager_C") (`self.S_HurtPlayer`) _returnvalue 1.0)
    (set `self.punchFlag` true)))

(fn `UserConstructionScript`)