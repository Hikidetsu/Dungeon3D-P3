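; BP_Turret is a turret that aims and fires at the third-person player character.
; When its PawnSensing component sees that character, it snaps its yaw toward the target, keeping pitch and roll level.
; After a short Delay, it spawns a BP_Proyectil at the Arrow component's transform and plays a shot sound.
; The Delay ignores repeat sightings while pending, so it also paces the firing.
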(event `self.PawnSensing.OnSeePawn`
  (params (Pawn :type "Pawn Object Reference"))
  ; ShootLogic
  (cast `/Game/ThirdPerson/Blueprints/BP_ThirdPersonCharacter` Pawn)
  (`self.K2_SetActorRotation` (`KismetMathLibrary.MakeRotator` 0.0 0.0 (.yaw (`KismetMathLibrary.FindLookAtRotation` (`self.K2_GetActorLocation`) (`self.K2_GetActorLocation` Pawn)))))
  (`KismetSystemLibrary.Delay` 1.0)
  (`|SpawnActorFromClass` "/Game/GameLogic/Characters/BP_Proyectil.BP_Proyectil_C" (`SceneComponent.K2_GetComponentToWorld` (`self.Arrow`)) "Undefined" "MultiplyWithRoot" null null)
  (`GameplayStatics.PlaySound2D` (`self.s_shoot`) 0.5 1.0 0.0 null null))

(fn `UserConstructionScript`)